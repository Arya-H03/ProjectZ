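; Timed grenade that explodes after its lifetime and kills BasicEnemy actors in the blast.
; A BeginPlay timer calls Explode, which enables overlap events on the Sphere and arms the grenade.
; A timeline then grows the sphere radius to sweep out the blast area.
; Any overlap while armed spawns the explosion emitter and destroys the grenade after a short delay, with enemies also receiving Death.
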(event `ExpandCollision`
  (set `self.canExplode` true)
  (bind (_direction _newtrack_0) (`Timeline|Timeline_0`)
    (:`Update`
      (`SphereComponent.SetSphereRadius` (`self.Sphere`) (`KismetMathLibrary.Lerp` 0.0 400.0 _newtrack_0) true))))

(event `self.ReceiveBeginPlay`
  (bind _returnvalue (`KismetSystemLibrary.K2_SetTimer` null "Explode" (`self.lifeTime`)))
  (set `self.remainingTime` _returnvalue))

(event `self.Sphere.OnComponentBeginOverlap`
  (params (OverlappedComponent :type "PrimitiveComponent Object Reference") (OtherActor :type "Actor Object Reference") (OtherComp :type "PrimitiveComponent Object Reference") (OtherBodyIndex :type Integer) (bFromSweep :type Boolean) (SweepResult :type "HitResult Structure (by ref)"))
  (bind _canexplode (`self.canExplode`))
  (bind _asbasic_enemy (cast `/Game/Enemies/BasicEnemy/BasicEnemy` OtherActor)
    (:`then`
      (if _canexplode
        (`/Game/Enemies/BasicEnemy/BasicEnemy.Death` _asbasic_enemy)
        (`GameplayStatics.SpawnEmitterAtLocation` "/Game/StarterContent/Particles/P_Explosion.P_Explosion" (`SceneComponent.K2_GetComponentLocation` (`self.StaticMesh`)) (struct) (4.0 4.0 4.0) :!label _label)
        (`KismetSystemLibrary.Delay` 0.11)
        (`self.K2_DestroyActor`)))
    (:`CastFailed`
      (if _canexplode
        (goto _label)))))

(fn `Explode`
  (set `PrimitiveComponent.bGenerateOverlapEvents` true (`self.Sphere`))
  (`self.ExpandCollision`))

(fn `UserConstructionScript`)