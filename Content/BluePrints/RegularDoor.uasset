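; RegularDoor is a sliding door that opens when BP_ThirdPersonCharacter enters its Box trigger and closes when the character leaves.
; A Timeline lerps the Cube from its BeginPlay location by the DoorOpenDirection offset, playing forward to open and reversing to close.
; Entering also hides the TextRender, plays a sound at the door and enables player input; leaving restores the text and disables input.
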(event `self.ReceiveBeginPlay`
  (set `self.initialLocation` (`SceneComponent.K2_GetComponentLocation` (`self.Cube`))))

(event `self.Box.OnComponentBeginOverlap`
  (params (OverlappedComponent :type "PrimitiveComponent Object Reference") (OtherActor :type "Actor Object Reference") (OtherComp :type "PrimitiveComponent Object Reference") (OtherBodyIndex :type Integer) (bFromSweep :type Boolean) (SweepResult :type "HitResult Structure (by ref)"))
  (bind _initiallocation (`self.initialLocation`))
  (cast `/Game/Player/BP_ThirdPersonCharacter` OtherActor)
  (`self.EnableInput` (`GameplayStatics.GetPlayerController` 0))
  (`SceneComponent.SetHiddenInGame` (`self.TextRender`) true false)
  (`GameplayStatics.PlaySoundAtLocation` null (`SceneComponent.K2_GetComponentLocation` (`self.Cube`)) (struct) 1.0 1.0 0.0 null null null null)
  (bind (_direction _0to1) (`Timeline|Timeline` :!label _label)
    (:`Update`
      (`SceneComponent.K2_SetWorldLocation` (`self.Cube`) (`KismetMathLibrary.VLerp` _initiallocation (+ _initiallocation (`self.doorOpenDirection`)) _0to1) false false))))

(event `self.Box.OnComponentEndOverlap`
  (params (OverlappedComponent :type "PrimitiveComponent Object Reference") (OtherActor :type "Actor Object Reference") (OtherComp :type "PrimitiveComponent Object Reference") (OtherBodyIndex :type Integer))
  (cast `/Game/Player/BP_ThirdPersonCharacter` OtherActor)
  (`self.DisableInput` (`GameplayStatics.GetPlayerController` 0))
  (`SceneComponent.SetHiddenInGame` (`self.TextRender`) false false)
  (goto _label :!via `Reverse`))

(fn `UserConstructionScript`)