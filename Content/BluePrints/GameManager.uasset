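; GameManager runs enemy waves around the player and brings in a boss once the kill target is met.
; SpawnEnemies, gated by CanSpawnEnemies, spawns random batches of Zombies and Parasites every ten seconds while the player lives.
; When EnemyKillCount reaches EnemyCount, the delayed loop ends and SpawnBoss spawns a Monster.
; All spawns use random X/Y offsets from the player's capsule and are added to EnemyList.
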(event `SpawnBoss`
  (bind (_returnvalue_x _returnvalue_y _returnvalue_z) (`KismetMathLibrary.BreakVector` (`SceneComponent.K2_GetComponentLocation` (`Character.CapsuleComponent` (`GameplayStatics.GetPlayerCharacter` 0)))))
  (bind _returnvalue (`|SpawnActorFromClass` "/Game/Enemies/Monster/Monster.Monster_C" (`KismetMathLibrary.MakeTransform` (`KismetMathLibrary.MakeVector` (+ _returnvalue_x (`KismetMathLibrary.RandomFloatInRange` -1000.0 1000.0)) (+ _returnvalue_y (`KismetMathLibrary.RandomFloatInRange` -1000.0 1000.0)) _returnvalue_z)) "Undefined" "OverrideRootScale" null null))
  (`KismetArrayLibrary.Array_Add` (`self.EnemyList`) _returnvalue)
  (`KismetSystemLibrary.PrintString` "Boss Has Spawned"))

(event `SpawnEnemies`
  (bind (_returnvalue_x _returnvalue_y _returnvalue_z) (`KismetMathLibrary.BreakVector` (`SceneComponent.K2_GetComponentLocation` (`Character.CapsuleComponent` (`GameplayStatics.GetPlayerCharacter` 0)))))
  (bind _returnvalue (+ _returnvalue_x (`KismetMathLibrary.RandomFloatInRange` -1000.0 1000.0)))
  (bind _returnvalue_2 (+ _returnvalue_y (`KismetMathLibrary.RandomFloatInRange` -1000.0 1000.0)))
  (if (`self.canSpawnEnemies`)
    (bind _asbp_third_person_character (cast `/Game/Player/BP_ThirdPersonCharacter` (`GameplayStatics.GetPlayerCharacter` 0)))
    (if (not (`/Game/Player/BP_ThirdPersonCharacter.isDead` _asbp_third_person_character)) :!label _label
      (for _ (range (+ (`KismetMathLibrary.RandomIntegerInRange` 6 10) 1))
        (bind _returnvalue_3 (`|SpawnActorFromClass` "/Game/Enemies/Zombie/Zombie.Zombie_C" (`KismetMathLibrary.MakeTransform` (`KismetMathLibrary.MakeVector` _returnvalue _returnvalue_2 _returnvalue_z)) "Undefined" "OverrideRootScale" null null))
        (`KismetArrayLibrary.Array_Add` (`self.EnemyList`) _returnvalue_3))
      (for _ (range (+ (`KismetMathLibrary.RandomIntegerInRange` 6 8) 1))
        (bind _returnvalue_4 (`|SpawnActorFromClass` "/Game/Enemies/Parasite/Parasite.Parasite_C" (`KismetMathLibrary.MakeTransform` (`KismetMathLibrary.MakeVector` _returnvalue _returnvalue_2 _returnvalue_z)) "Undefined" "OverrideRootScale" null null))
        (`KismetArrayLibrary.Array_Add` (`self.EnemyList`) _returnvalue_4))
      (`KismetSystemLibrary.Delay` 10.0)
      (if (< (`self.enemyKillCount`) (`self.enemyCount`))
        (goto _label)
        (else
          (`self.SpawnBoss`))))))

(fn `UserConstructionScript`)