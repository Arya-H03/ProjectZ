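; SpawnActivator is a trigger actor that starts an enemy challenge when the third-person character first overlaps its box.
; The overlap clears CanStart and sets a five-second timer to enable and call enemy spawning on the GameManager found in the level.
; After a one-second delay, it switches off its spotlight, turns the listed level lights bright red and updates its text render.
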(event `self.Box.OnComponentBeginOverlap`
  (params (OverlappedComponent :type "PrimitiveComponent Object Reference") (OtherActor :type "Actor Object Reference") (OtherComp :type "PrimitiveComponent Object Reference") (OtherBodyIndex :type Integer) (bFromSweep :type Boolean) (SweepResult :type "HitResult Structure (by ref)"))
  (if (`self.canStart`)
    (cast `/Game/Player/BP_ThirdPersonCharacter` OtherActor)
    (`self.StartChallenge`)))

(event `StartChallenge`
  (bind _returnvalue (`KismetSystemLibrary.K2_SetTimer` null "SpawnEnemies" 5.0))
  (set `self.Time` _returnvalue)
  (set `self.canStart` false)
  (`KismetSystemLibrary.Delay` 1.0)
  (`LightComponent.SetIntensity` (`self.SpotLight`) 0.0)
  (for _array_element (`self.levelLights`)
    (bind _pointlightcomponent (`PointLight.PointLightComponent` _array_element))
    (`LightComponent.SetIntensity` _pointlightcomponent 1000.0)
    (`LightComponent.SetLightColor` _pointlightcomponent (struct :`R` 0.796875 :`A` 1.0) true)
    (`LightComponent.SetIntensity` (`self.SpotLight`) 0.0)
    (`TextRenderComponent.K2_SetText` (`self.TextRender`) (`self.Value`))))

(event `SpawnEnemies`
  (bind _returnvalue (`GameplayStatics.GetActorOfClass` "/Game/BluePrints/GameManager.GameManager_C"))
  (set `/Game/BluePrints/GameManager.canSpawnEnemies` true _returnvalue)
  (`/Game/BluePrints/GameManager.SpawnEnemies` _returnvalue))

(fn `UserConstructionScript`)